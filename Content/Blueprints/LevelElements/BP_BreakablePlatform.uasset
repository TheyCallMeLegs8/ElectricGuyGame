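; Breakable platform actor that disappears a few seconds after something overlaps its Box trigger, then reappears.
; A chain of Delays spawns an explosion effect at the Cube, hides the actor and disables Cube collision, then calls Respawn to restore both.
; The overlap has no actor filter, and its Broken guard is only set just before Respawn clears it.
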(event OnComponentBeginOverlap(Box)
  (params (OverlappedComponent :type Primitive%20Component%20Object%20Reference) (OtherActor :type Actor%20Object%20Reference) (OtherComp :type Primitive%20Component%20Object%20Reference) (OtherBodyIndex :type Integer) (bFromSweep :type Boolean) (SweepResult :type Hit%20Result%20Structure%20%28by%20ref%29))
  (if (not (Variables|Default|Get_Broken))
    (bind _output_get (Variables|Default|Set_IsHidden true))
    (Utilities|FlowControl|Delay 1.5)
    (Niagara|SpawnSystematLocation "/Game/Art/Emitters/E_Explosion.E_Explosion" (Transformation|GetWorldLocation (Variables|Default|GetCube)))
    (Utilities|FlowControl|Delay 1.5)
    (Rendering|SetActorHiddenInGame _output_get)
    (Collision|SetCollisionEnabled (Variables|Default|GetCube) "NoCollision")
    (Utilities|FlowControl|Delay 3.0)
    (Variables|Default|Set_Broken true)
    (CallFunction|Respawn)))

(event Custom|Respawn
  (if (Variables|Default|Get_IsHidden)
    (Variables|Default|Set_IsHidden false)
    (Rendering|SetActorHiddenInGame false)
    (Collision|SetCollisionEnabled (Variables|Default|GetCube) "QueryAndPhysics")
    (Variables|Default|Set_Broken false)))

(fn ConstructionScript)