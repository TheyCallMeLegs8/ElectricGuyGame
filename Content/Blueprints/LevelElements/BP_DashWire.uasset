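; BP_DashWire is a spline-shaped wire level element, with overlap detection that so far only prints a debug message.
; The construction script adds a spline mesh component between each pair of spline points, aligned on X using local locations and tangents.
; Each segment overwrites the single SplineMesh variable, so BeginPlay binds the overlap handler only to the last segment.
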(event Custom|OnSplineMeshCollide
  (params (OverlappedComponent :type Primitive%20Component%20Object%20Reference) (OtherActor :type Actor%20Object%20Reference) (OtherComp :type Primitive%20Component%20Object%20Reference) (OtherBodyIndex :type Integer) (bFromSweep :type Boolean) (SweepResult :type Hit%20Result%20Structure%20%28by%20ref%29))
  (Development|PrintString "Collided with Spline Mesh"))

(event EventBeginPlay
  (Collision|BindEventtoOnComponentBeginOverlap (Variables|Default|GetSplineMesh) (delegate Custom|OnSplineMeshCollide)))

(event Collision|EventActorBeginOverlap
  (params (OtherActor :type Actor%20Object%20Reference)))

(event EventTick
  (params (DeltaSeconds :type Float%20%28single-precision%29)))

(fn ConstructionScript
  (bind _spline (Variables|Default|GetSpline))
  ;[1 1 1] Aligns spline mesh along spline
  (for _index (range 0 (- (Spline|GetNumberOfSplinePoints (Variables|Default|GetSpline)) 2))
    (bind _returnvalue (AddComponent|AddSplineMeshComponent false))
    (bind _output_get (Variables|Default|SetSplineMesh _returnvalue))
    (SplineMesh|SetForwardAxis _output_get "X" true)
    (SplineMesh|SetStartandEnd _output_get (Spline|GetLocationatSplinePoint _spline _index "Local") (Spline|GetTangentatSplinePoint _spline _index "Local") (Spline|GetLocationatSplinePoint _spline (+ _index 1) "Local") (Spline|GetTangentatSplinePoint _spline (+ _index 1) "Local") true :!class /Script/Engine.SplineMeshComponent)))