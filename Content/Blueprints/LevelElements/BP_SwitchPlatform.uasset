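; BP_SwitchPlatform is a level element pairing an overlap-triggered switch with a platform that it moves.
; When anything begins overlapping the Box, a timeline rotates the StaticMesh toward a target rotation, setting IsFlipped and calling Flipped on every update.
; Flipped plays a second timeline that lerps the Platform's relative location from its local zero to a target offset, without sweep.
; The graph has no reverse or reset path.
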(event OnComponentBeginOverlap(Box)
  (params (OverlappedComponent :type Primitive%20Component%20Object%20Reference) (OtherActor :type Actor%20Object%20Reference) (OtherComp :type Primitive%20Component%20Object%20Reference) (OtherBodyIndex :type Integer) (bFromSweep :type Boolean) (SweepResult :type Hit%20Result%20Structure%20%28by%20ref%29))
  (bind _rotate (Timeline|Timeline Play)
    (:Update
      (Transformation|SetRelativeRotation (Variables|Default|GetStaticMesh) (Math|Rotator|Lerp(Rotator) "0, 0, 0" (Variables|Default|GetB_0) _rotate) false false)
      (Variables|Default|SetIsFlipped true)
      (CallFunction|Flipped))))

(event Custom|Flipped
  (if (Variables|Default|GetIsFlipped)
    (bind _moving_platform (Timeline|Timeline_0 Play)
      (:Update
        (Transformation|SetRelativeLocation (Variables|Default|GetPlatform) (Math|Vector|Lerp(Vector) "0, 0, 0" (Variables|Default|GetB) _moving_platform) false false)))))

(fn ConstructionScript)