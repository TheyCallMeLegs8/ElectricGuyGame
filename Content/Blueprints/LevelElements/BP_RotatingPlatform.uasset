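; BP_RotatingPlatform is a level platform that flips between two rotations each time the player dashes.
; On BeginPlay it finds the player character actors and binds its Dashing event to their OnPlayerDash dispatcher.
; Dashing checks IsFlipped to play one of two timelines, which lerp RotatePoint's relative rotation toward NewRotation or ReRotation and update the flag.
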(event Custom|Dashing
  (if (Variables|Default|Get_IsFlipped)
    (bind _rerotate (Timeline|RotationReflip Play)
      (:Update
        (Transformation|SetRelativeRotation (Variables|Default|GetRotatePoint) (Math|Rotator|Lerp(Rotator) "0, 0, 0" (Variables|Default|Get_ReRotation) _rerotate) false false)
        (Variables|Default|Set_IsFlipped false)))
    (else
      (bind _rotation (Timeline|Rotation Play)
        (:Update
          (Transformation|SetRelativeRotation (Variables|Default|GetRotatePoint) (Math|Rotator|Lerp(Rotator) "0, 0, 0" (Variables|Default|Get_NewRotation) _rotation) false false)
          (Variables|Default|Set_IsFlipped true))))))

(event EventBeginPlay
  (bind _outactors (Actor|GetAllActorsOfClass "/Game/Blueprints/Character/Player/BP_PlayerCharacter.BP_PlayerCharacter_C")) ; Getting reference of Player character
  (EventDispatchers|AssignOnPlayerDash _outactors (delegate Custom|Dashing)))

(fn ConstructionScript)